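; BP_FloorButton2 is an interactable floor button with a hieroglyph symbol that toggles on and off.
; Trigger zone overlaps track whether a Character is on it, enabling the IA_Interact input.
; Each press alternates through a FlipFlop that sets IsOn, swaps the symbol's ON/OFF material, calls the OnPressedChanged dispatcher and prints the state.
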(event `self.TriggerZone.OnComponentBeginOverlap`
  (params (OverlappedComponent :type "PrimitiveComponent Object Reference") (OtherActor :type "Actor Object Reference") (OtherComp :type "PrimitiveComponent Object Reference") (OtherBodyIndex :type Integer) (bFromSweep :type Boolean) (SweepResult :type "HitResult Structure (by ref)"))
  (cast `Character` OtherActor)
  (set `self.bPlayerOnButton` true))

(event `EnhancedInput|/Game/00_Examen_UNIR/Input/Actions/IA_Interact`
  (params (ActionValue :type Boolean) (ElapsedSeconds :type "Float (double-precision)") (TriggeredSeconds :type "Float (double-precision)") (InputAction :type "InputAction Object Reference" :default "/Game/00_Examen_UNIR/Input/Actions/IA_Interact.IA_Interact"))
  (:`Started`
    (if (`self.bPlayerOnButton`)
      (`/Engine/EditorBlueprintResources/StandardMacros.FlipFlop`
        (:`A`
          (set `self.bIsOn` true)
          (`PrimitiveComponent.SetMaterial` (`self.HieroglyphSymbol`) 0 (`self.MatON`))
          (`self.OnPressedChanged`)
          (`KismetSystemLibrary.PrintString` "Button ON"))
        (:`B`
          (set `self.bIsOn` false)
          (`PrimitiveComponent.SetMaterial` (`self.HieroglyphSymbol`) 0 (`self.MatOFF`))
          (`self.OnPressedChanged`)
          (`KismetSystemLibrary.PrintString` "Button OFF"))))))

(event `self.TriggerZone.OnComponentEndOverlap`
  (params (OverlappedComponent :type "PrimitiveComponent Object Reference") (OtherActor :type "Actor Object Reference") (OtherComp :type "PrimitiveComponent Object Reference") (OtherBodyIndex :type Integer))
  (cast `Character` OtherActor)
  (set `self.bPlayerOnButton` false))

(fn `UserConstructionScript`)