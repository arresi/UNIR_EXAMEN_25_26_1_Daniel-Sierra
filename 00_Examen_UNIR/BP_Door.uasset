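; Door Blueprint that opens when all of its linked Buttons are on and closes when any turns off.
; BeginPlay binds to each button's pressed-changed event and runs an initial check of all buttons.
; State changes toggle IsOpen, playing one timeline from start to open and reversing a separate one to close.
; Lerp-based Y-offset moves in opposite directions exist, but their nodes are unreachable as wired.
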(event `self.ReceiveBeginPlay`
  (for _ (`self.Buttons`)
    (add `/Game/00_Examen_UNIR/BP_FloorButton.OnPressedChanged` (`|CreateDelegate` :!event `CheckAllButtons`)))
  (`self.CheckAllButtons`))

(event `CheckAllButtons`
  (set `self.bAllPressed` true)
  (for _ (`self.Buttons`)
    (if (not (`/Game/00_Examen_UNIR/BP_FloorButton.bIsOn`))
      (set `self.bAllPressed` false)))
  (if (`self.bAllPressed`)
    (if (not (`self.bIsOpen`))
      (`self.OpenDoor`))
    (elif (`self.bIsOpen`)
      (`self.CloseDoor`))))

(event `OpenDoor`
  (set `self.bIsOpen` true)
  (`Timeline|Cronograma` :!via `PlayFromStart`))

(event `CloseDoor`
  (set `self.bIsOpen` false)
  (`Timeline|Cronograma_0` :!via `Reverse`))

(fn `UserConstructionScript`)